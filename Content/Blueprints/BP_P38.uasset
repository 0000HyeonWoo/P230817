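; BP_P38 is a player-controlled plane pawn with roll and pitch steering, boost and a rocket launcher.
; Axis inputs rotate it locally, while Tick adds movement input scaled by Boost (Left Shift), though its direction is zero and the forward vector is unconnected.
; BPRotateActorComponent spins both propellers.
; Left Ctrl fires through BPSpawnActorComponent at the Rocket's transform, using its cleared mesh as a cooldown gate until a delay restores it.
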(event EventBeginPlay
  ;[1 1 1] Add Rotate Component
  (Default|AddSceneComponents (Variables|Default|GetBP_RotateActorComponent) (Variables|Default|GetRightPropeller))
  (Default|AddSceneComponents (Variables|Default|GetBP_RotateActorComponent) (Variables|Default|GetLeftPropeller))
  ;[1 1 1] Rotate Axis
  (Variables|/Game/Blueprints/BP_RotateActorComponent.BP_RotateActorComponent_C|SetAxis (Variables|Default|GetBP_RotateActorComponent) "0.000000,0.000000,1.000000")
  (Default|AddSceneComponent (Variables|Default|GetBP_SpawnActorComponent) (Variables|Default|GetRocket)))

(event EventTick
  (params (DeltaSeconds :type Float%20%28single-precision%29))
  ;[1 1 1] FloatingPawnMovement - Forward
  (Pawn|Input|AddMovementInput "0, 0, 0" (Variables|Default|GetBoost) false))

(event Input|ActionEvents|InputActionLeftShift
  (params (Key :type Key%20Structure :default "None"))
  ;[1 1 1] Boost
  (:Pressed
    (Variables|Default|SetBoost 1.0))
  (:Released
    (Variables|Default|SetBoost 0.5)))

(event Input|ActionEvents|InputActionLeftCtrl
  (params (Key :type Key%20Structure :default "None"))
  ;[1 1 1] Launch Rocket
  (:Pressed
    ;;[1 1 1] RocketMesh IsValid
    (Utilities|IsValid (Variables|/Script/Engine.StaticMeshComponent|GetStaticMesh (Variables|Default|GetRocket))
      (:Is%20Valid
        (Default|SpawnActor (Variables|Default|GetBP_SpawnActorComponent) (Transformation|GetWorldTransform (Variables|Default|GetRocket)))
        ;;[1 1 1] Reload
        (Components|StaticMesh|SetStaticMesh (Variables|Default|GetRocket) 0)
        ;;;[1 1 1] Reload Cooltime
        (Utilities|FlowControl|Delay 3.0)
        (Components|StaticMesh|SetStaticMesh (Variables|Default|GetRocket) "/Game/Meshs/SM_Rocket.SM_Rocket")))))

(event Input|AxisEvents|InputAxisRoll
  (params (AxisValue :type Float%20%28single-precision%29))
  ;[1 1 1] Roll Input
  (Transformation|AddActorLocalRotation (Math|Rotator|MakeRotator (* AxisValue (Variables|Default|GetRotateSpeed) (Utilities|Time|GetWorldDeltaSeconds)) 0.0 0.0) false false))

(event Input|AxisEvents|InputAxisPitch
  (params (AxisValue :type Float%20%28single-precision%29))
  ;[1 1 1] Pitch Input
  (Transformation|AddActorLocalRotation (Math|Rotator|MakeRotator 0.0 (* AxisValue (Variables|Default|GetRotateSpeed) (Utilities|Time|GetWorldDeltaSeconds)) 0.0) false false))

(fn ConstructionScript)