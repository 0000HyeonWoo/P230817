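; BP_RotateActorComponent is an actor component that continuously spins a registered set of scene components.
; AddSceneComponents appends components to its internal array.
; Each Tick, every component in the array receives a local rotation of Axis times Speed, scaled by world delta seconds for frame-rate independence.
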(event EventTick
  (params (DeltaSeconds :type Float%20%28single-precision%29))
  ;[1 1 1] Rotate SceneComponent
  (for _array_element (Variables|Default|GetSceneComponent)
    (Transformation|AddLocalRotation _array_element (* (* (Variables|Default|GetAxis) (Variables|Default|GetSpeed)) (Utilities|Time|GetWorldDeltaSeconds)) false false)))

(fn AddSceneComponents
  (params (NewComponent :type Scene%20Component%20Object%20Reference%20%28by%20ref%29))
  (Utilities|Array|Add (Variables|Default|GetSceneComponent) NewComponent))